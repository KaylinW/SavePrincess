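; EnemyBP is an enemy actor that travels the length of a spline path in the level.
; On BeginPlay it looks up a SplinePathBP actor and starts a timeline whose play rate is the inverse of TimeToComplete.
; Each timeline update maps the track value to a distance along the spline and moves the actor there without sweeping.
; The transform is built from location alone, so the actor does not rotate to follow the path.
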(event `self.ReceiveBeginPlay`
  (bind _returnvalue (`GameplayStatics.GetActorOfClass` "/Game/Blueprints/SplinePathBP.SplinePathBP_C"))
  (set `self.SplineRef` _returnvalue)
  (`self.Move Object`))

(event `Move Object`
  (`TimelineComponent.SetPlayRate` (`self.Move Object T`) (/ 1.0 (`self.TimeToComplete`)))
  (bind (_direction _movetrack) (`Timeline|Move Object T`)
    (:`Update`
      (`self.K2_SetActorTransform` (`KismetMathLibrary.Conv_VectorToTransform` (`SplineComponent.GetLocationAtDistanceAlongSpline` (`/Game/Blueprints/SplinePathBP.Spline` (`self.SplineRef`)) (`KismetMathLibrary.Lerp` 0.0 (`SplineComponent.GetSplineLength` (`/Game/Blueprints/SplinePathBP.Spline` (`self.SplineRef`))) _movetrack) "World"))))))

(fn `UserConstructionScript`)